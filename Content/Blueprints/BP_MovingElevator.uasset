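; Elevator Blueprint that moves a Platform between Start and End transforms when BP_ThirdPersonCharacter overlaps its trigger volumes.
; While IsMovingUp is true, the End trigger plays a Timeline from the start and the Start trigger reverses it.
; The Timeline lerps platform location and rotation, swapping its material between moving and stopped.
; IsMovingUp is never set here, and a duplicate Timeline_0 chain is unconnected.
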(event `self.Start Trigger.OnComponentBeginOverlap`
  (params (OverlappedComponent :type "PrimitiveComponent Object Reference") (OtherActor :type "Actor Object Reference") (OtherComp :type "PrimitiveComponent Object Reference") (OtherBodyIndex :type Integer) (bFromSweep :type Boolean) (SweepResult :type "HitResult Structure (by ref)"))
  ; Comment
  (`KismetSystemLibrary.PrintString` "You hit the elevator Start Trigger")
  (if (`self.IsMovingUp`)
    (cast `/Game/ThirdPerson/Blueprints/BP_ThirdPersonCharacter` OtherActor)
    (`self.Activate Start Trigger`)))

(event `CustomEvent`
  ;[0.07824 0.05469 0.375 0.5] BP_MovingPlatform Blueprint (EXAMPLE
)

(event `self.End Trigger.OnComponentBeginOverlap`
  (params (OverlappedComponent :type "PrimitiveComponent Object Reference") (OtherActor :type "Actor Object Reference") (OtherComp :type "PrimitiveComponent Object Reference") (OtherBodyIndex :type Integer) (bFromSweep :type Boolean) (SweepResult :type "HitResult Structure (by ref)"))
  ; Comment
  (`KismetSystemLibrary.PrintString` "You hit the elevator End Trigger")
  (if (`self.IsMovingUp`)
    (cast `/Game/ThirdPerson/Blueprints/BP_ThirdPersonCharacter` OtherActor)
    (`self.Activate End Trigger`)))

(event `Activate Start Trigger`
  (bind (_direction _newtrack_0) (`Timeline|Timeline` :!via `Reverse` :!label _label)
    (:`Update`
      (bind (_returnvalue_location _returnvalue_rotation) (`KismetMathLibrary.BreakTransform` (`KismetMathLibrary.TLerp` (`SceneComponent.K2_GetComponentToWorld` (`self.Start`)) (`SceneComponent.K2_GetComponentToWorld` (`self.End`)) _newtrack_0)))
      (`SceneComponent.K2_SetWorldLocationAndRotation` (`self.Platform`) _returnvalue_location _returnvalue_rotation false false))
    (:`Moving`
      (`PrimitiveComponent.SetMaterial` (`self.Platform`) 0 "/Game/LevelPrototyping/Materials/MI_Solid_Blue.MI_Solid_Blue"))
    (:`Stopped`
      (`PrimitiveComponent.SetMaterial` (`self.Platform`) 0 "/Game/StarterContent/Materials/M_AssetPlatform.M_AssetPlatform"))))

(event `Activate End Trigger`
  (goto _label :!via `PlayFromStart`))

(fn `UserConstructionScript`)