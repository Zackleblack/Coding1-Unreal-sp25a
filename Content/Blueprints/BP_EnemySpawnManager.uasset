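; BP_EnemySpawnManager is an early-stage manager for enemy waves that so far only prints debug messages.
; BeginPlay reports the number of BP_EnemySpawner actors in the level, with a placeholder in place of the enemy count.
; NewEnemyWaveCHeck prints whether any BP_Enemy actors remain.
; SpawnNewEnemies announces a four-second spawn but runs only a short delay and spawns nothing.
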(event `self.ReceiveBeginPlay`
  (`KismetSystemLibrary.PrintString` "Spawn Manager is active")
  (bind _outactors (`GameplayStatics.GetAllActorsOfClass` "/Game/Blueprints/BP_EnemySpawner.BP_EnemySpawner_C"))
  (`KismetSystemLibrary.PrintString` (`KismetStringLibrary.Concat_StrStr` "There are" (`KismetStringLibrary.Conv_IntToString` (`KismetArrayLibrary.Array_Length` _outactors)) "Spawners in the level" "There are " "##" "Enemies in the level") true true (struct :`R` 0.252778 :`G` 0.230999 :`B` 1.0 :`A` 1.0)))

(event `NewEnemyWaveCHeck`
  (`KismetSystemLibrary.PrintString` "Checking enemy count")
  (bind _outactors (`GameplayStatics.GetAllActorsOfClass` "/Game/Blueprints/BP_Enemy.BP_Enemy_C"))
  (if (> (`KismetArrayLibrary.Array_Length` _outactors) 0)
    (`KismetSystemLibrary.PrintString` "There are still monsters")))

(event `Spawn New Enemies`
  (`KismetSystemLibrary.PrintString` "spawning new enemies in 4 seconds" true true (struct :`R` 1.0 :`G` 0.321716 :`B` 0.858572 :`A` 1.0) 5.0)
  (`KismetSystemLibrary.Delay` 0.2))

(fn `UserConstructionScript`)